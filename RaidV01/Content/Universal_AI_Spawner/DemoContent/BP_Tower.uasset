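; BP_Tower is a demo defense tower for the Universal AI Spawner that destroys non-player pawns entering its range.
; On the server, Sphere1 overlaps add and remove pawns in a Targets list and start a looping Fire timer at the reload interval.
; Fire traces from the Sphere component to the first target with debug drawing, destroys the pawn it hits, and clears the timer when no valid target remains.
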(event OnComponentBeginOverlap(Sphere1)
  (params (OverlappedComponent :type Primitive%20Component%20Object%20Reference) (OtherActor :type Actor%20Object%20Reference) (OtherComp :type Primitive%20Component%20Object%20Reference) (OtherBodyIndex :type Integer) (bFromSweep :type Boolean) (SweepResult :type Hit%20Result%20Structure%20%28by%20ref%29))
  (Networking|SwitchHasAuthority
    (:Authority
      (bind _aspawn (Utilities|Casting|CastToPawn OtherActor))
      (Utilities|IsValid _aspawn
        (:Is%20Valid
          (if (not (Class|Controller|IsPlayerController (Pawn|GetController _aspawn)))
            (Utilities|Array|Add (Variables|Default|GetTargets) _aspawn)
            (if (not (Utilities|Time|IsTimerActivebyHandle (Variables|Default|GetTimer_Fire)))
              (bind _returnvalue (Utilities|Time|SetTimerbyFunctionName 0 "Fire" (Variables|Default|GetReloadTime) true))
              (Variables|Default|SetTimer_Fire _returnvalue))))))))

(event OnComponentEndOverlap(Sphere1)
  (params (OverlappedComponent :type Primitive%20Component%20Object%20Reference) (OtherActor :type Actor%20Object%20Reference) (OtherComp :type Primitive%20Component%20Object%20Reference) (OtherBodyIndex :type Integer))
  (Networking|SwitchHasAuthority
    (:Authority
      (bind _aspawn (Utilities|Casting|CastToPawn OtherActor))
      (Utilities|IsValid _aspawn
        (:Is%20Valid
          (Utilities|Array|RemoveItem (Variables|Default|GetTargets) _aspawn))))))

(event EventBeginPlay)

(event Collision|EventActorBeginOverlap
  (params (OtherActor :type Actor%20Object%20Reference)))

(event EventTick
  (params (DeltaSeconds :type Float%20%28single-precision%29)))

(fn ConstructionScript)

(fn Fire
  (bind _targets (Variables|Default|GetTargets))
  (bind _output (Utilities|Array|Get(acopy) _targets))
  (Networking|SwitchHasAuthority
    (:Authority
      (Utilities|IsValid _output
        (:Is%20Valid
          (bind _outhit (Collision|LineTraceForObjects (Transformation|GetWorldLocation (Variables|Default|GetSphere)) (Transformation|GetActorLocation _output) (Utilities|Array|MakeArray "ObjectTypeQuery3") false 0 "ForDuration" true "(R=1.000000,G=0.000000,B=0.000000,A=1.000000)" "(R=0.000000,G=1.000000,B=0.000000,A=1.000000)" 1.0))
          (bind _aspawn (Utilities|Casting|CastToPawn (.HitActor (Collision|BreakHitResult _outhit))))
          (Actor|DestroyActor _aspawn))
        (:Is%20Not%20Valid
          (Utilities|Time|ClearandInvalidateTimerbyHandle (Variables|Default|GetTimer_Fire)))))))

(fn Reload
  (Variables|Default|SetReadyToFire true))