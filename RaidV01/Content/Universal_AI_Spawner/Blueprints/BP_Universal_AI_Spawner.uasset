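; Box-volume AI spawner that places pawns on the server, instantly or with random delays, and can run behavior trees on them.
; The construction script precomputes spawn points using random or seeded sphere traces, retrying on blocked actors, misses or steep slopes.
; Destroyed pawns respawn at newly traced points with optional per-entry limits.
; In wave mode, clearing pawns instead advances to the next wave after a pause or fires the end event.
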(event Custom|Respawn_Event
  (params (Str_SpawnInfo :type Spawn%20Info%20Structure%20%28by%20ref%29) (Index :type Integer))
  (bind (_spawnclass _count _behaviortree _scale) (Utilities|Struct|BreakSpawnInfo Str_SpawnInfo))
  ;[1 1 1] Respawn Event
  (if (not (Variables|Default|GetStopSpawn))
    (Utilities|FlowControl|Sequence
      (:then_0
        (if (Variables|CommonSettings|GetUseRespawnLimits?)
          (if (> (Utilities|Array|Get(acopy) (Variables|Default|GetRespawnLimit) Index) 0)
            (Variables|Default|SetStopRespawn false)
            (else
              (Variables|Default|SetStopRespawn true)))
          (else
            (Variables|Default|SetStopRespawn false))))
      (:then_1
        (if (not (Variables|Default|GetStopRespawn))
          (bind (_success _location) (CallFunction|CheckLocation Str_SpawnInfo))
          (if _success
            (bind _returnvalue (Game|SpawnActorfromClass _spawnclass (Math|Transform|MakeTransform _location (select (Variables|CommonSettings|GetRandomZRotation) (Math|Rotator|MakeRotator 0.0 0.0 (Math|Random|RandomFloatinRange -1.8e+02 1.8e+02)) (Variables|CommonSettings|GetRotation)) (Math|Conversions|ToVector(Float) _scale)) "AdjustIfPossibleButAlwaysSpawn" 0 0))
            (Utilities|Array|Add (Variables|Default|GetSpawnedPawns) _returnvalue)
            (Utilities|FlowControl|Sequence
              (:then_0
                (if (Variables|CommonSettings|GetRespawn?)
                  (Utilities|Array|Add (Variables|Default|GetRespawnInfo) (Utilities|Struct|MakePawnInfo Index _returnvalue)))
                (Game|BindEventtoOnDestroyed _returnvalue (delegate Custom|ActorDestroyed)))
              (:then_1
                (Utilities|IsValid 0
                  (:Is%20Valid
                    (AI|RunBehaviorTree (AI|GetAIController _returnvalue)))))
              (:then_2
                (if (Variables|CommonSettings|GetUseRespawnLimits?)
                  (Utilities|Array|SetArrayElem (Variables|Default|GetRespawnLimit) Index (- (Utilities|Array|Get(acopy) (Variables|Default|GetRespawnLimit) Index) 1)))))))))))

(event Custom|ActorDestroyed
  (params (DestroyedActor :type Actor%20Object%20Reference))
  ;[1 1 1] Bind Pawn Event Destroyed
  (bind _aspawn (Utilities|Casting|CastToPawn DestroyedActor))
  (Variables|Default|SetSuccess false)
  (Utilities|Array|RemoveItem (Variables|Default|GetSpawnedPawns) _aspawn)
  (if (and (Variables|CommonSettings|GetRespawn?) (not (Variables|WavesModeSettings|GetWavesMode?)))
    (bind (_array_element _array_index) (Utilities|Array|ForEachLoopwithBreak (Variables|Default|GetRespawnInfo) :!label _label)
      (:LoopBody
        (if (== _aspawn (.Pawn (Utilities|Struct|BreakPawnInfo _array_element)))
          (Variables|Default|SetPawnIndex (.PawnIndex (Utilities|Struct|BreakPawnInfo _array_element)))
          (Variables|Default|SetSuccess true)
          (Utilities|Array|RemoveIndex (Variables|Default|GetRespawnInfo) _array_index)
          (goto _label Break)))
      (:Completed
        (if (Variables|Default|GetSuccess) :!label _label_2
          (CallFunction|RespawnEvent (Utilities|Array|Get(acopy) (Variables|CommonSettings|GetSpawnAI_Info) (Variables|Default|GetPawnIndex)) (Variables|Default|GetPawnIndex)))
        (if (Variables|WavesModeSettings|GetWavesMode?)
          (bind _success (CallFunction|ChecktoEndWave))
          (if _success
            (if (select (Variables|WavesModeSettings|GetUse_"SpawnAI_Info"_AsWaves?) (>= (Variables|Default|GetSpawnInfoIndex) (- (Utilities|Array|Length (Variables|CommonSettings|GetSpawnAI_Info)) 1)) (>= (Variables|Default|GetWaveCurrent) (Variables|WavesModeSettings|GetWavesLimit)))
              (CallFunction|-WavesEndEvent)
              (else
                (Utilities|FlowControl|Delay (Variables|WavesModeSettings|GetPauseForNextWave))
                (Math|Integer|IncrementInt (Variables|Default|GetWaveCurrent)
                  (:%20%20
                    (if (Variables|WavesModeSettings|GetUse_"SpawnAI_Info"_AsWaves?)
                      (Math|Integer|IncrementInt (Variables|Default|GetSpawnInfoIndex)
                        (:%20%20
                          _))
                      (else
                        (Variables|Default|SetSpawnInfoIndex 0)))
                    (CallFunction|SetRespawnLimits)
                    (CallFunction|StartSpawn)))))))))
    (else
      (goto _label_2))))

(event Custom|CustomStartSpawn
  ;[1 1 1] Custom Start Spawn
  (if (not (Variables|Default|GetSpawned))
    (Variables|Default|SetSpawned true)
    (CallFunction|StartSpawn)))

(event Custom|-WavesEndEvent
  ;[0 0.1576 1] END WAVES - USE FOR YOU EVENTS
)

(event Custom|Spawn
  (bind _locationforspawn (Variables|Default|GetLocationForSpawn))
  (bind _use__spawnai_info__aswaves_ (Variables|WavesModeSettings|GetUse_"SpawnAI_Info"_AsWaves?))
  ;[1 1 1] Spawn Event
  (if (not (Variables|Default|GetStopSpawn))
    (if _use__spawnai_info__aswaves_
      (for _index (range 0 (- (.Count (Utilities|Struct|BreakSpawnInfo (select _use__spawnai_info__aswaves_ (Utilities|Array|Get(acopy) (Variables|CommonSettings|GetSpawnAI_Info) (Variables|Default|GetSpawnInfoIndex)) (stale _array_element)))) 1)) :!label _label
        (if (Utilities|Array|IsValidIndex _locationforspawn _index)
          (bind _returnvalue (Game|SpawnActorfromClass (.SpawnClass (Utilities|Struct|BreakSpawnInfo (select _use__spawnai_info__aswaves_ (Utilities|Array|Get(acopy) (Variables|CommonSettings|GetSpawnAI_Info) (Variables|Default|GetSpawnInfoIndex)) (stale _array_element)))) (Math|Transform|MakeTransform (.location (Utilities|Array|Get(acopy) _locationforspawn _index)) (select (Variables|CommonSettings|GetRandomZRotation) (Math|Rotator|MakeRotator 0.0 0.0 (Math|Random|RandomFloatinRange -1.8e+02 1.8e+02)) (Variables|CommonSettings|GetRotation)) (Math|Conversions|ToVector(Float) (.Scale (Utilities|Struct|BreakSpawnInfo (select _use__spawnai_info__aswaves_ (Utilities|Array|Get(acopy) (Variables|CommonSettings|GetSpawnAI_Info) (Variables|Default|GetSpawnInfoIndex)) (stale _array_element)))))) "AdjustIfPossibleButAlwaysSpawn" 0 0))
          (Utilities|Array|Add (Variables|Default|GetSpawnedPawns) _returnvalue)
          (Utilities|FlowControl|Sequence
            (:then_0
              (if (Variables|CommonSettings|GetRespawn?)
                (Utilities|Array|Add (Variables|Default|GetRespawnInfo) (Utilities|Struct|MakePawnInfo (Variables|Default|GetSpawnInfoIndex) _returnvalue)))
              (Game|BindEventtoOnDestroyed _returnvalue (delegate Custom|ActorDestroyed)))
            (:then_1
              (Utilities|IsValid 0
                (:Is%20Valid
                  (AI|RunBehaviorTree (AI|GetAIController _returnvalue))))))))
      (else
        (for (_array_element _array_index) (Variables|CommonSettings|GetSpawnAI_Info)
          (Variables|Default|SetSpawnInfoIndex _array_index)
          (goto _label))))))

(event Custom|-WavesEndGameOver
  ;[0 0.1576 1] END WAVES - USE FOR YOU EVENTS
  (Variables|Default|SetStopSpawn true))

(event Custom|SpawnWithDelay
  (bind _spawnai_info (Variables|CommonSettings|GetSpawnAI_Info))
  (bind _spawninfoindex (Variables|Default|GetSpawnInfoIndex))
  (bind _spawnwithdelay_ (Variables|CommonSettings|GetSpawnWithDelay_))
  (bind (_spawnwithdelay__2 _min _max) (Utilities|Struct|BreakSpawnWithDelay _spawnwithdelay_))
  (bind _output (Utilities|Array|Get(acopy) _spawnai_info _spawninfoindex))
  (bind (_spawnclass _count _behaviortree _scale) (Utilities|Struct|BreakSpawnInfo _output))
  ;[1 1 1] Spawn With Delay
  (if (not (Variables|Default|GetStopSpawn))
    (bind _output_get (Variables|Default|SetIndex _count :!label _label))
    (if (!= (- _output_get 1) -1)
      (bind _returnvalue (Game|SpawnActorfromClass _spawnclass (Math|Transform|MakeTransform (.location (Utilities|Array|Get(acopy) (Variables|Default|GetLocationForSpawn) (- _output_get 1))) (select (Variables|CommonSettings|GetRandomZRotation) (Math|Rotator|MakeRotator 0.0 0.0 (Math|Random|RandomFloatinRange -1.8e+02 1.8e+02)) (Variables|CommonSettings|GetRotation)) (Math|Conversions|ToVector(Float) _scale)) "AdjustIfPossibleButAlwaysSpawn" 0 0 :!label _label_2))
      (Utilities|Array|Add (Variables|Default|GetSpawnedPawns) _returnvalue)
      (Utilities|FlowControl|Sequence
        (:then_0
          (if (Variables|CommonSettings|GetRespawn?)
            (Utilities|Array|Add (Variables|Default|GetRespawnInfo) (Utilities|Struct|MakePawnInfo (Variables|Default|GetSpawnInfoIndex) _returnvalue)))
          (Game|BindEventtoOnDestroyed _returnvalue (delegate Custom|ActorDestroyed)))
        (:then_1
          (Utilities|IsValid _behaviortree
            (:Is%20Valid
              (AI|RunBehaviorTree (AI|GetAIController _returnvalue) _behaviortree))))
        (:then_2
          (bind _output_get_2 (Variables|Default|SetIndex (- (Variables|Default|GetIndex) 1)))
          (if (<= _output_get_2 0)
            (if (< (Variables|Default|GetSpawnInfoIndex) (- (Utilities|Array|Length (Variables|CommonSettings|GetSpawnAI_Info)) 1))
              (if (not (Variables|WavesModeSettings|GetUse_"SpawnAI_Info"_AsWaves?))
                (Math|Integer|IncrementInt (Variables|Default|GetSpawnInfoIndex)
                  (:%20%20
                    (goto _label)))))
            (else
              (Utilities|FlowControl|Delay (Math|Random|RandomFloatinRange _min _max))
              (goto _label_2))))))))

(event Custom|StartSpawn
  ;[1 1 1] Start Spawn
  ;;[0 0.1221 1] Use With Event To Custom Spawn with Link
  (Utilities|FlowControl|Delay (Variables|CommonSettings|GetStartSpawnDelay))
  (Utilities|Array|Clear (Variables|Default|GetRespawnInfo))
  (if (Utilities|Struct|BreakSpawnWithDelay (Variables|CommonSettings|GetSpawnWithDelay_))
    (CallFunction|SpawnwithDelay)
    (else
      (CallFunction|Spawn))))

(event EventBeginPlay
  ;[1 1 1] Begin Play
  (Networking|SwitchHasAuthority
    (:Authority
      (Utilities|FlowControl|Delay 1.5)
      (CallFunction|SetRespawnLimits)
      (if (not (Variables|CommonSettings|GetStopStartSpawn_%28CustomSpawn%29?))
        (CallFunction|StartSpawn)))))

(fn ConstructionScript
  (bind _arrow (Variables|Default|GetArrow))
  (Math|Random|SetRandomStreamSeed (Variables|Default|GetStream) (Variables|CommonSettings|GetStreamSeed))
  (Components|Box|SetBoxExtent (Variables|Default|GetBox) (Variables|CommonSettings|GetSpawnBox) true)
  (Transformation|SetRelativeRotation _arrow (Variables|CommonSettings|GetRotation) false false)
  (Transformation|SetRelativeLocation _arrow (Math|Vector|MakeVector 0.0 0.0 (.Z (Math|Vector|BreakVector (Variables|CommonSettings|GetSpawnBox)))) false false)
  (CallFunction|SpawnPreview)
  (if (Variables|WavesModeSettings|GetUse_"SpawnAI_Info"_AsWaves?)
    (Variables|WavesModeSettings|SetWavesMode? true)))

(fn SpawnPreview
  (Utilities|Array|Clear (Variables|Default|GetLocationForSpawn))
  (Rendering|Debug|FlushPersistentDebugLines)
  (for _array_element (Variables|CommonSettings|GetSpawnAI_Info)
    (for _index (range 0 (- (.Count (Utilities|Struct|BreakSpawnInfo _array_element)) 1))
      (LocalVariables|Setlocal_Index _index)
      (LocalVariables|Setlocal_InfLoop 0)
      (bind (_success _location) (CallFunction|CheckLocation _array_element))
      (if _success
        (Utilities|Array|SetArrayElem (Variables|Default|GetLocationForSpawn) _index (Utilities|Struct|MakeLocation _location) true)
        (if (Variables|CommonSettings|GetShowDebugSphere?)
          (Rendering|Debug|DrawDebugSphere _location (.SpawnSphereRadius (Utilities|Struct|BreakSpawnInfo _array_element)) 12 "(R=0.154764,G=1.000000,B=0.000000,A=1.000000)" 999999.0))))))

(fn FindRandomPointinBox
  (bind _spawnbox (Variables|CommonSettings|GetSpawnBox))
  (bind (_x _y) (Math|Vector|BreakVector _spawnbox))
  (return (select (Variables|CommonSettings|GetStream?) (+ (CallFunction|FindRandomPointStream (Variables|Default|GetStream)) (Transformation|GetActorLocation)) (Math|Random|RandomPointinBoundingBox (Transformation|GetActorLocation) (Math|Vector|MakeVector _x _y 0.0)))))

(fn FindRandomPointStream
  (params (Stream :type Random%20Stream%20Structure%20%28by%20ref%29))
  (bind _spawnbox (Variables|CommonSettings|GetSpawnBox))
  (bind (_x _y) (Math|Vector|BreakVector _spawnbox))
  (bind _returnvalue (* _spawnbox -1.0))
  (bind (_x_2 _y_2) (Math|Vector|BreakVector _returnvalue))
  (return (Math|Vector|MakeVector (Math|Random|RandomFloatinRangefromStream _x_2 _x Stream) (Math|Random|RandomFloatinRangefromStream _y_2 _y Stream) 0.0)))

(fn CheckLocation
  (params (SpawnInfo :type Spawn%20Info%20Structure))
  (bind _spawnbox (Variables|CommonSettings|GetSpawnBox))
  (bind _z (Math|Vector|BreakVector _spawnbox))
  (bind _output_get (LocalVariables|Setlocal_Point (CallFunction|FindRandomPointinBox) :!label _label))
  (bind _outhit (Collision|SphereTraceByChannel (Math|Vector|MakeVector (.X (Math|Vector|BreakVector _output_get)) (.Y (Math|Vector|BreakVector _output_get)) (+ (.Z (Math|Vector|BreakVector _output_get)) _z)) (Math|Vector|MakeVector (.X (Math|Vector|BreakVector _output_get)) (.Y (Math|Vector|BreakVector _output_get)) (- (.Z (Math|Vector|BreakVector _output_get)) _z)) (Utilities|Struct|BreakSpawnInfo SpawnInfo) (Variables|CommonSettings|GetSpawnTraceChannel) false 0 "None"))
  (if (Utilities|Array|ContainsItem (Variables|CommonSettings|GetBlockSpawnActors) (.HitActor (Collision|BreakHitResult _outhit)))
    _
    (elif (Math|Vector|Equal(Vector) (.Location (Collision|BreakHitResult _outhit)) "0, 0, 0" 0.1)
      _
      (elif (>= (Variables|CommonSettings|GetInclineAngleMax) (Class|KismetMathLibrary|DegAcos (Math|Vector|DotProduct (.ImpactNormal (Collision|BreakHitResult _outhit)) "0, 0,1.000000")))
        (return true (.Location (Collision|BreakHitResult _outhit)))
        (else
          _))))
  (bind _result (Math|Integer|IncrementInt (LocalVariables|Getlocal_InfLoop))
    (:%20%20
      (if (< _result 50)
        (goto _label)
        (else
          (return false "0, 0, 0"))))))

(fn SetRespawnLimits
  (Utilities|Array|Clear (Variables|Default|GetRespawnLimit))
  (for _array_element (Variables|CommonSettings|GetSpawnAI_Info)
    (Utilities|Array|Add (Variables|Default|GetRespawnLimit) (.RespawnLimit (Utilities|Struct|BreakSpawnInfo _array_element)))))

(fn ChecktoEndWave
  (Utilities|FlowControl|Sequence
    (:then_0
      (if (Variables|CommonSettings|GetUseRespawnLimits?)
        (if (Variables|WavesModeSettings|GetUse_"SpawnAI_Info"_AsWaves?)
          (if (> (Utilities|Array|Get(acopy) (Variables|Default|GetRespawnLimit) (Variables|Default|GetSpawnInfoIndex)) 0)
            (LocalVariables|Setlocal_Success false))
          (else
            (bind _array_element (Utilities|Array|ForEachLoopwithBreak (Variables|Default|GetRespawnLimit) :!label _label)
              (:LoopBody
                (if (> _array_element 0)
                  (LocalVariables|Setlocal_Success false)
                  (goto _label Break))))))))
    (:then_1
      (if (not (== (Utilities|Array|Length (Variables|Default|GetSpawnedPawns)) 0))
        (LocalVariables|Setlocal_Success false)))
    (:then_2
      (return (LocalVariables|Getlocal_Success)))))