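; BP_TriggerWaveCounter is a wave-defense trigger volume that tracks how many pawns get through before the player loses.
; Any pawn overlapping its box is destroyed and lowers a remaining count shown on a TextRender.
; At zero it calls WavesEndGameOver on the referenced Spawner and shows a lose message.
; The construction script sizes the box and initializes the counter text in the editor.
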(event OnComponentBeginOverlap(Box)
  (params (OverlappedComponent :type Primitive%20Component%20Object%20Reference) (OtherActor :type Actor%20Object%20Reference) (OtherComp :type Primitive%20Component%20Object%20Reference) (OtherBodyIndex :type Integer) (bFromSweep :type Boolean) (SweepResult :type Hit%20Result%20Structure%20%28by%20ref%29))
  (bind _aspawn (Utilities|Casting|CastToPawn OtherActor))
  (Actor|DestroyActor _aspawn)
  (bind _output_get (Variables|Default|SetCountForEndGame (Math|Integer|Max(Integer) (- (Variables|Default|GetCountForEndGame) 1))))
  (if (<= _output_get 0)
    (Default|-WavesEndGameOver (Variables|Default|GetSpawner))
    (Rendering|Components|TextRender|SetText (Variables|Default|GetTextRender) (Utilities|Text|FormatText "YOU LOSE"))
    (else
      (Rendering|Components|TextRender|SetText (Variables|Default|GetTextRender) (Utilities|Text|FormatText "COUNT FOR LOSE: {Count}" _output_get)))))

(event EventBeginPlay)

(event Collision|EventActorBeginOverlap
  (params (OtherActor :type Actor%20Object%20Reference)))

(event EventTick
  (params (DeltaSeconds :type Float%20%28single-precision%29)))

(fn ConstructionScript
  (Components|Box|SetBoxExtent (Variables|Default|GetBox) (Variables|Default|GetBoxExtent) true)
  (Rendering|Components|TextRender|SetText (Variables|Default|GetTextRender) (Utilities|Text|FormatText "COUNT FOR LOSE: {Count}" (Variables|Default|GetCountForEndGame))))