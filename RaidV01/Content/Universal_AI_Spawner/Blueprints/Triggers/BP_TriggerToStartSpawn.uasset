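; Trigger volume actor that starts a referenced AI Spawner when a player walks into it.
; Box overlap passes the other actor to a server-named event, which casts it to Pawn and checks for a PlayerController before calling CustomStartSpawn on the Spawner.
; The construction script sizes the box from the BoxExtent variable.
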(event OnComponentBeginOverlap(Box)
  (params (OverlappedComponent :type Primitive%20Component%20Object%20Reference) (OtherActor :type Actor%20Object%20Reference) (OtherComp :type Primitive%20Component%20Object%20Reference) (OtherBodyIndex :type Integer) (bFromSweep :type Boolean) (SweepResult :type Hit%20Result%20Structure%20%28by%20ref%29))
  (CallFunction|StartSpawnSERVER OtherActor))

(event Custom|StartSpawn_SERVER
  (params (Actor :type Actor%20Object%20Reference))
  (bind _aspawn (Utilities|Casting|CastToPawn Actor))
  (if (Class|Controller|IsPlayerController (Pawn|GetController _aspawn))
    (Default|CustomStartSpawn (Variables|Default|GetSpawner))))

(fn ConstructionScript
  (Components|Box|SetBoxExtent (Variables|Default|GetBox) (Variables|Default|GetBoxExtent) true))