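; Behavior tree task that makes an enemy attack a pawn in front of it.
; On execution it casts the controlled pawn to EnemyCharacterBase and sphere-traces a short distance along its forward vector for Pawn objects.
; A hit passes the actor to PerformAttack and finishes the task as failed.
; A miss or failed cast never calls FinishExecute.
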(event EventReceiveExecuteAI
  (params (OwnerController :type AI%20Controller%20Object%20Reference) (ControlledPawn :type Pawn%20Object%20Reference))
  (bind _asenemy_character_base (Utilities|Casting|CastToEnemyCharacterBase ControlledPawn))
  (bind (_outhit _returnvalue) (Collision|SphereTraceForObjects (Transformation|GetActorLocation _asenemy_character_base) (+ (Transformation|GetActorLocation _asenemy_character_base) (* (Math|Vector|GetForwardVector (Transformation|GetActorRotation _asenemy_character_base)) 2.5e+02)) 1.2e+02 (Utilities|Array|MakeArray "ObjectTypeQuery3") false 0 "None"))
  (if _returnvalue
    (Class|EnemyCharacterBase|PerformAttack _asenemy_character_base (.HitActor (Collision|BreakHitResult _outhit)))
    (AI|BehaviorTree|FinishExecute false)))