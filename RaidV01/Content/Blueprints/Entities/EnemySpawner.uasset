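; Enemy spawner actor that spawns AI pawns of EnemyTemplate at its own location, using the SpawnType mode chosen at BeginPlay.
; Delay mode spawns on a DelayTimer loop, while Dump mode re-triggers itself at a short fixed interval; both destroy the actor when EnemyCount reaches zero.
; Respawn mode spawns once after a brief delay and clears IsAlive, with its EnemyCount update left unconnected and no respawn logic in these graphs.
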(event Custom|spawnDump
  (Utilities|FlowControl|Delay 0.15)
  (CallFunction|Spawn)
  (bind _result (Math|Integer|DecrementInt (Variables|Default|GetenemyCount))
    (:%20%20
      (bind _output_get (Variables|Default|SetenemyCount _result))
      (if (== _output_get 0)
        (Actor|DestroyActor)
        (else
          (CallFunction|SpawnDump))))))

(event Custom|spawnRespawn
  (Utilities|FlowControl|Delay 0.05)
  (CallFunction|Spawn)
  (bind _result (Math|Integer|DecrementInt (Variables|Default|GetenemyCount))
    (:%20%20
      (Variables|Default|SetisAlive false))))

(event Custom|spawnDelay
  (Utilities|FlowControl|Delay (Variables|Default|GetdelayTimer) :!label _label)
  (CallFunction|Spawn)
  (bind _result (Math|Integer|DecrementInt (Variables|Default|GetenemyCount))
    (:%20%20
      (bind _output_get (Variables|Default|SetenemyCount _result))
      (if (== _output_get 0)
        (Actor|DestroyActor)
        (else
          (goto _label))))))

(event Custom|spawn
  (AI|SpawnAIFromClass (Variables|Default|GetenemyTemplate) 0 (Transformation|GetWorldLocation (Variables|Default|GetDefaultSceneRoot)) "0, 0, 0" false 0))

(event EventBeginPlay
  (switch Utilities|FlowControl|Switch|SwitchonspawnType (Variables|Default|GetspawnType)
    (:NewEnumerator0
      (CallFunction|SpawnDelay))
    (:NewEnumerator1
      (CallFunction|SpawnRespawn))
    (:NewEnumerator2
      (CallFunction|SpawnDump))))

(fn ConstructionScript)