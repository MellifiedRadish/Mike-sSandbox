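; BP_Menu3D is a 3D main-menu screen actor with a widget component that pans the view to linked menus.
; Its widget's PanToMenu event selects a LinkedMenus entry by index, then swaps collision to that actor and blends the view target to it.
; The current widget hides during the eased blend, and the destination's appears once it finishes.
; If the widget is the main menu, BeginPlay also assigns JigglySquares as button backgrounds.
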(event Custom|PanTo
  (params (NewMenu :type BP%20Menu%203D%20Object%20Reference))
  (bind _widget (Variables|BP_Menu3D_C|GetWidget NewMenu))
  (Rendering|SetVisibility (Variables|Default|GetWidget) false true)
  (Collision|SetActorEnableCollision false)
  (Collision|SetActorEnableCollision NewMenu true)
  (Game|Player|SetViewTargetwithBlend (Game|GetPlayerController 0) NewMenu 1.75 "VTBlend_EaseInOut" 2.0 false)
  (Utilities|FlowControl|Delay 1.75)
  (Rendering|SetVisibility _widget true true)
  (Rendering|SetCastShadow _widget false))

(event Custom|OnEvent_PanToMenu
  (params (MenuIndex :type Integer))
  (if (Utilities|Array|IsValidIndex (Variables|Default|GetLinkedMenus) MenuIndex)
    (CallFunction|Panto (Utilities|Array|Get(acopy) (Variables|Default|GetLinkedMenus) MenuIndex))))

(event EventBeginPlay
  (bind _jigglysquares (Variables|Default|GetJigglySquares))
  (bind _asbp_menu_3dwidget (Utilities|Casting|CastToBP_Menu3DWidget (UserInterface|GetUserWidgetObject (Variables|Default|GetWidget))))
  (EventDispatchers|AssignPantoMenu _asbp_menu_3dwidget (delegate Custom|OnEvent_PanToMenu))
  (Collision|SetActorEnableCollision false)
  (bind _asbp_main_menu_widget (Utilities|Casting|CastToBP_MainMenuWidget (UserInterface|GetUserWidgetObject (Variables|Default|GetWidget))))
  (Variables|/Game/Blueprints/MainMenu/Widgets/BP_ButtonWidget.BP_ButtonWidget_C|SetBackgroundObj (Variables|/Game/Blueprints/MainMenu/Widgets/BP_MainMenuWidget.BP_MainMenuWidget_C|GetPlayButton _asbp_main_menu_widget) (Utilities|Array|Get(acopy) _jigglysquares))
  (Variables|/Game/Blueprints/MainMenu/Widgets/BP_ButtonWidget.BP_ButtonWidget_C|SetBackgroundObj (Variables|/Game/Blueprints/MainMenu/Widgets/BP_MainMenuWidget.BP_MainMenuWidget_C|GetSettingsButton _asbp_main_menu_widget) (Utilities|Array|Get(acopy) _jigglysquares 1))
  (Variables|/Game/Blueprints/MainMenu/Widgets/BP_ButtonWidget.BP_ButtonWidget_C|SetBackgroundObj (Variables|/Game/Blueprints/MainMenu/Widgets/BP_MainMenuWidget.BP_MainMenuWidget_C|GetCreditsButton _asbp_main_menu_widget) (Utilities|Array|Get(acopy) _jigglysquares 2))
  (Variables|/Game/Blueprints/MainMenu/Widgets/BP_ButtonWidget.BP_ButtonWidget_C|SetBackgroundObj (Variables|/Game/Blueprints/MainMenu/Widgets/BP_MainMenuWidget.BP_MainMenuWidget_C|GetQuitButton _asbp_main_menu_widget) (Utilities|Array|Get(acopy) _jigglysquares 3)))

(fn ConstructionScript)